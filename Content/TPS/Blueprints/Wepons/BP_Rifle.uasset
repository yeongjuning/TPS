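; Rifle weapon Blueprint that extends a parent weapon class with hitscan firing.
; On FireandAttack it runs the parent logic, then, if ammo is not empty, reads range and damage from the "Weapon1" data table row.
; It line-traces forward from the muzzle socket on the Visibility channel with timed debug drawing.
; A hit applies point damage and reports a damage event, the hook used by AI damage sensing.
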(event EventBeginPlay
  (|CallParentFunction))

(event Collision|EventActorBeginOverlap
  (params (OtherActor :type Actor%20Object%20Reference))
  (|CallParentFunction OtherActor) ; 지금 이 노드는 비활성 상태입니다. \n핀을 끌어서 다른 노드를 연결하면 활성화됩니다.
)

(event EventTick
  (params (DeltaSeconds :type Float%20%28single-precision%29))
  (|CallParentFunction DeltaSeconds) ; 지금 이 노드는 비활성 상태입니다. \n핀을 끌어서 다른 노드를 연결하면 활성화됩니다.
)

(event EventFireandAttack
  (bind _returnvalue (Game|GetInstigatorController))
  (bind _mesh (Variables|Character|GetMesh))
  (bind _returnvalue_2 (Transformation|GetSocketTransform _mesh "Socket_Muzzle" "RTS_World"))
  (bind (_location _rotation) (Math|Transform|BreakTransform _returnvalue_2))
  (|CallParentFunction)
  (if (not (Class|WeaponBase|IsAmmoEmpty))
    (bind _returnvalue_3 (Utilities|GetDataTableRow "/Game/TPS/DataTables/WeaponDataTable.WeaponDataTable" "Weapon1")
      (:then
        (bind (_outhit _returnvalue_4) (Collision|LineTraceByChannel _location (+ (* (Math|Vector|GetForwardVector _rotation) (.attackrange _returnvalue_3)) _location) "TraceTypeQuery1" false 0 "ForDuration" true "(R=1.000000,G=0.000000,B=0.000000,A=1.000000)" "(R=0.000000,G=1.000000,B=0.000000,A=1.000000)" 6.0))
        (if _returnvalue_4
          (bind _returnvalue_5 (Game|Damage|ApplyPointDamage (.HitActor (Collision|BreakHitResult _outhit)) (.basedamage _returnvalue_3) (.Normal (Collision|BreakHitResult _outhit)) _outhit _returnvalue self))
          (Class|AISenseDamage|ReportDamageEvent (.HitActor (Collision|BreakHitResult _outhit)) _returnvalue _returnvalue_5 (.Location (Collision|BreakHitResult _outhit))))))))

(fn ConstructionScript
  (|CallParentFunction))