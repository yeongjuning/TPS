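; AI controller for TPS enemies that runs their behavior tree and tracks the player through AI perception.
; Sensing a Player-tagged actor cancels the loss timer and writes line-of-sight and follow target to the blackboard.
; Any other perception update starts a one-shot timer that clears both keys on expiry, giving a grace period before the enemy drops its target.
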(event OnTargetPerceptionUpdated(AIPerception)
  (params (Actor :type Actor%20Object%20Reference) (Stimulus :type AI%20Stimulus%20Structure))
  ;[1 1 1] 나중에 C++ 코드로 짜기
  (if (and (Actor|ActorHasTag Actor "Player") (.bSuccessfullySensed (Utilities|Struct|BreakAIStimulus Stimulus)))
    (Development|PrintString "Player감지")
    ;;[1 1 1] Player가 감지 되었을 때
    (Utilities|Time|ClearandInvalidateTimerbyHandle (Variables|Default|GetEnemyTimerHandle))
    (AI|Components|Blackboard|SetValueasBool (AI|GetBlackboard self) (Variables|Default|GetHasLineOfSight) true)
    (AI|Components|Blackboard|SetValueasObject (AI|GetBlackboard self) (Variables|Default|GetTargetToFollow) Actor)
    (else
      (Development|PrintString "Player 미감지")
      ;;[1 1 1] Player가 감지 되었는데 몇초 이상 안보일때
      (bind _returnvalue (Utilities|Time|SetTimerbyEvent (delegate Custom|StartEnemyTimer) (Variables|Default|GetGameTimer)))
      (Variables|Default|SetEnemyTimerHandle _returnvalue))))

(event Custom|StartEnemyTimer
  (bind _returnvalue (AI|GetBlackboard 0))
  ;[1 1 1] 나중에 C++ 코드로 짜기
  ;;[1 1 1] Player가 감지 되었는데 몇초 이상 안보일때
  (AI|Components|Blackboard|SetValueasBool _returnvalue (Variables|Default|GetHasLineOfSight) false)
  (AI|Components|Blackboard|SetValueasObject _returnvalue (Variables|Default|GetTargetToFollow) 0))

(event EventBeginPlay
  ;[1 1 1] 나중에 C++ 코드로 짜기
  (Utilities|FlowControl|Sequence
    (:then_0
      (Class|AIController|UseBlackboard "/Game/TPS/Blueprints/Enemys/AI/BB_EnemyAI.BB_EnemyAI"))
    (:then_1
      (AI|RunBehaviorTree "/Game/TPS/Blueprints/Enemys/AI/BT_EnemyAI.BT_EnemyAI"))))

(event EventTick
  (params (DeltaSeconds :type Float%20%28single-precision%29))
  ;[1 1 1] 나중에 C++ 코드로 짜기
)

(fn ConstructionScript)